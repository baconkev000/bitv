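; One-time interactable chest that animates its lid and a dissolving sphere, then grants a health, attack or speed boost, or turns the player into an alien.
; Overlapping its box shows an interact widget; Interact plays the timelines, applies the reward, shows a notification and increments Brain_BP's chest count.
; Alien odds rise with that count past a threshold.
; The normal reward roll only completes when all three stats are below maximum.
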(event OnComponentBeginOverlap(Box)
  (params (OverlappedComponent :type Primitive%20Component%20Object%20Reference) (OtherActor :type Actor%20Object%20Reference) (OtherComp :type Primitive%20Component%20Object%20Reference) (OtherBodyIndex :type Integer) (bFromSweep :type Boolean) (SweepResult :type Hit%20Result%20Structure%20%28by%20ref%29))
  ;[1 1 1] Interact Widget
  (if (not (Variables|Default|GetHasBeenOpened))
    (Rendering|SetVisibility (Variables|Default|GetWidget) true false)))

(event OnComponentEndOverlap(Box)
  (params (OverlappedComponent :type Primitive%20Component%20Object%20Reference) (OtherActor :type Actor%20Object%20Reference) (OtherComp :type Primitive%20Component%20Object%20Reference) (OtherBodyIndex :type Integer))
  ;[1 1 1] Interact Widget
  (Rendering|SetVisibility (Variables|Default|GetWidget) false false))

(event Custom|Get%20Brain%20Ref
  (bind _outactors (Actor|GetAllActorsOfClass "/Game/Levels/Brain_BP.Brain_BP_C"))
  (Variables|Default|SetBrainRef (Utilities|Array|Get(acopy) _outactors)))

(event EventBeginPlay
  (CallFunction|GetBrainRef))

(event EventInteract
  (params (InteractingActor :type Actor%20Object%20Reference))
  (bind _rewardtype (Variables|Default|GetRewardType))
  (bind _returnvalue (Utilities|String|EnumtoString _rewardtype))
  (Variables|Default|SetInteractingPlayer InteractingActor)
  (if (not (Variables|Default|GetHasBeenOpened))
    (Utilities|FlowControl|Sequence
      (:then_0
        (bind _chestfloat (Timeline|OpenChest%20Timeline Play)
          (:Update
            (Utilities|FlowControl|Sequence
              (:then_0
                (Transformation|SetRelativeLocation (Variables|Default|Getchest_lid) (Math|Vector|MakeVector 0.0 0.0 (Math|Float|Lerp -3e+01 1.1e+02 _chestfloat)) false false))
              (:then_1
                ;[1 1 1] Sphere Animations
                (bind _spherefloat (Timeline|RotateSphereTimeline Play)
                  (:Update
                    (Utilities|FlowControl|Sequence
                      (:then_0
                        (Transformation|SetRelativeRotation (Variables|Default|GetBP_sphere) (Math|Rotator|MakeRotator (Math|Float|Lerp 0.0 9e+02 _spherefloat) (Math|Float|Lerp 0.0 9e+02 _spherefloat) (Math|Float|Lerp 0.0 9e+02 _spherefloat)) false false))
                      (:then_1
                        (Transformation|SetRelativeLocation (Variables|Default|GetBP_sphere) (Math|Vector|MakeVector 0.0 0.0 (Math|Float|Lerp 0.0 1e+02 _chestfloat)) false false))
                      (:then_2
                        (bind _asbp_sphere (Utilities|Casting|CastToBP_sphere (Variables|/Script/Engine.ChildActorComponent|GetChildActor (Variables|Default|GetBP_sphere))))
                        (Default|StartDissolve _asbp_sphere))))))))))
      (:then_1
        ;[1 1 1] Chest Rewards
        (bind _asbp_third_person_character (Utilities|Casting|CastToBP_ThirdPersonCharacter (Variables|Default|GetInteractingPlayer)))
        (bind _reward (CallFunction|GetReward))
        (switch Utilities|FlowControl|Switch|SwitchonERewardType _reward
          (:NewEnumerator0
            (Default|IncreasePlayerHealth _asbp_third_person_character)
            (bind _asbp_sphere_2 (Utilities|Casting|CastToBP_sphere (Variables|/Script/Engine.ChildActorComponent|GetChildActor (Variables|Default|GetBP_sphere))))
            (Default|SetHealthColor _asbp_sphere_2)
            (bind _returnvalue_2 (UserInterface|CreateWidget "/Game/Widgets/W_PlayerNotificatin.W_PlayerNotificatin_C"))
            (Default|UpdateRewardText _returnvalue_2 _returnvalue (Variables|/Game/ThirdPerson/Blueprints/BP_ThirdPersonCharacter.BP_ThirdPersonCharacter_C|GetHealthMultiplyer _asbp_third_person_character))
            (UserInterface|Viewport|AddtoViewport _returnvalue_2 0)
            (Utilities|FlowControl|Delay 2.0)
            (Widget|RemovefromParent _returnvalue_2))
          (:NewEnumerator1
            (Default|IncreasePlayerAttack _asbp_third_person_character)
            (bind _asbp_sphere_3 (Utilities|Casting|CastToBP_sphere (Variables|/Script/Engine.ChildActorComponent|GetChildActor (Variables|Default|GetBP_sphere))))
            (Default|SetAttackColor _asbp_sphere_3)
            (bind _returnvalue_3 (UserInterface|CreateWidget "/Game/Widgets/W_PlayerNotificatin.W_PlayerNotificatin_C"))
            (Default|UpdateRewardText _returnvalue_3 _returnvalue (Variables|/Game/ThirdPerson/Blueprints/BP_ThirdPersonCharacter.BP_ThirdPersonCharacter_C|GetAttackMultiplyer _asbp_third_person_character))
            (UserInterface|Viewport|AddtoViewport _returnvalue_3 0)
            (Utilities|FlowControl|Delay 2.0)
            (Widget|RemovefromParent _returnvalue_3))
          (:NewEnumerator2
            (Default|IncreasePlayerSpeed _asbp_third_person_character)
            (bind _asbp_sphere_4 (Utilities|Casting|CastToBP_sphere (Variables|/Script/Engine.ChildActorComponent|GetChildActor (Variables|Default|GetBP_sphere))))
            (Default|SetSpeedColor _asbp_sphere_4)
            (bind _returnvalue_4 (UserInterface|CreateWidget "/Game/Widgets/W_PlayerNotificatin.W_PlayerNotificatin_C"))
            (Default|UpdateRewardText _returnvalue_4 _returnvalue (Variables|/Game/ThirdPerson/Blueprints/BP_ThirdPersonCharacter.BP_ThirdPersonCharacter_C|GetSpeedMultiplyer _asbp_third_person_character))
            (UserInterface|Viewport|AddtoViewport _returnvalue_4 0)
            (Utilities|FlowControl|Delay 2.0)
            (Widget|RemovefromParent _returnvalue_4))
          (:NewEnumerator3
            (bind _asplayer_controller (Utilities|Casting|CastToPlayerController (Pawn|GetController _asbp_third_person_character)))
            (Actor|DestroyActor _asbp_third_person_character)
            (bind _returnvalue_5 (Game|SpawnActorfromClass "/Game/ThirdPerson/Blueprints/BP_TurnedAlien.BP_TurnedAlien_C" (Transformation|GetActorTransform _asplayer_controller) "Undefined" "MultiplyWithRoot" 0 0))
            (Pawn|Possess _asplayer_controller _returnvalue_5)
            (bind _returnvalue_6 (UserInterface|CreateWidget "/Game/Widgets/W_PlayerNotificatin.W_PlayerNotificatin_C"))
            (Default|UpdateNotificationText _returnvalue_6 "YOU ARE NOW THE ALIEN"))))
      (:then_2
        (Rendering|SetVisibility (Variables|Default|GetWidget) false false)
        (Variables|Default|SetHasBeenOpened true))
      (:then_3
        (Audio|PlaySoundatLocation "/Game/Chest/Chest.Chest" "0, 0, 0" "0, 0, 0" 1.0 1.0 0.0 0 0 0 0))
      (:then_4
        (Default|IncreaseChestsOpened (Variables|Default|GetBrainRef))))))

(fn ConstructionScript)

(fn GetReward
  (bind _brainref (Variables|Default|GetBrainRef))
  (bind _chestsopened (Variables|/Game/Levels/Brain_BP.Brain_BP_C|GetChestsOpened _brainref))
  (if (< _chestsopened (Variables|Default|GetChestsOpenedBeforAlien))
    (Variables|Default|SetAlienChance 0.0)
    (bind _reward (CallFunction|GetRewardType))
    (return _reward)
    (else
      (bind _output_get (Variables|Default|SetAlienChance (Math|Float|Clamp(Float) (* (Math|Conversions|ToFloat(Integer) (- _chestsopened (Variables|Default|GetChestsOpenedBeforAlien))) (Variables|Default|GetAlienChancePercent)))))
      (if (>= _output_get (Math|Random|RandomFloatinRange 0.0 1.0))
        (bind _output_get_2 (Variables|Default|SetRewardType "NewEnumerator3"))
        (return _output_get_2)
        (else
          (bind _reward_2 (CallFunction|GetRewardType))
          (return _reward_2))))))

(fn GetRewardType
  (bind _output_get (Variables|Default|SetEligableRewards (Utilities|Array|MakeArray "NewEnumerator0")))
  (Utilities|Array|Clear _output_get)
  (bind _asbp_third_person_character (Utilities|Casting|CastToBP_ThirdPersonCharacter (Variables|Default|GetInteractingPlayer)))
  (if (not (== (Variables|/Game/ThirdPerson/Blueprints/BP_ThirdPersonCharacter.BP_ThirdPersonCharacter_C|GetHealth _asbp_third_person_character) (Variables|/Game/ThirdPerson/Blueprints/BP_ThirdPersonCharacter.BP_ThirdPersonCharacter_C|GetMaxAllowedHealth _asbp_third_person_character)))
    (Utilities|Array|Add (Variables|Default|GetEligableRewards) "NewEnumerator0")
    (if (not (== (Variables|/Game/ThirdPerson/Blueprints/BP_ThirdPersonCharacter.BP_ThirdPersonCharacter_C|GetPlayerAttack _asbp_third_person_character) (Variables|/Game/ThirdPerson/Blueprints/BP_ThirdPersonCharacter.BP_ThirdPersonCharacter_C|GetMaxAllowedAttack _asbp_third_person_character)))
      (Utilities|Array|Add (Variables|Default|GetEligableRewards) "NewEnumerator1")
      (if (not (== (Variables|/Script/Engine.CharacterMovementComponent|GetMaxWalkSpeed (Variables|/Script/Engine.Character|GetCharacterMovement _asbp_third_person_character)) (Variables|/Game/ThirdPerson/Blueprints/BP_ThirdPersonCharacter.BP_ThirdPersonCharacter_C|GetMaxAllowedSpeed _asbp_third_person_character)))
        (Utilities|Array|Add (Variables|Default|GetEligableRewards) "NewEnumerator2")
        (bind _output_get_2 (Variables|Default|SetRewardType (Utilities|Array|Get(acopy) (Variables|Default|GetEligableRewards) (Math|Random|RandomIntegerinRange 0 (- (Utilities|Array|Length (Variables|Default|GetEligableRewards)) 1)))))
        (return _output_get_2)))))