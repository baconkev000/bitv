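; BP_sphere is a chest-related visual actor made of a sphere and two tori that can be tinted by type and dissolved.
; On BeginPlay it creates a dynamic instance of Dissolve_Inst for each of the three meshes.
; Attack, health and speed events set a red, green or yellow EmissionColor on all three materials.
; StartDissolve plays a timeline that drives their Dissolve scalar together.
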(event Custom|SetAttackColor
  (Rendering|Material|SetVectorParameterValue (stale EventBeginPlay _output_get) "EmissionColor" "(R=1.000000,G=0.218125,B=0.247975,A=1.000000)" :!class /Script/Engine.MaterialInstanceDynamic))

(event Custom|SetHealthColor
  (Rendering|Material|SetVectorParameterValue (stale EventBeginPlay _output_get) "EmissionColor" "(R=0.113636,G=0.552083,B=0.000000,A=1.000000)" :!class /Script/Engine.MaterialInstanceDynamic))

(event Custom|StartDissolve
  (bind _dissolvevallue (Timeline|DisolveTimeline Play)
    (:Update
      (Utilities|FlowControl|Sequence
        (:then_0
          (Rendering|Material|SetScalarParameterValue (Variables|Default|GetDM_Sphere) "Dissolve" _dissolvevallue :!class /Script/Engine.MaterialInstanceDynamic))
        (:then_1
          (Rendering|Material|SetScalarParameterValue (Variables|Default|GetDM_torus_1) "Dissolve" _dissolvevallue :!class /Script/Engine.MaterialInstanceDynamic))
        (:then_2
          (Rendering|Material|SetScalarParameterValue (Variables|Default|GetDM_Torus_2) "Dissolve" _dissolvevallue :!class /Script/Engine.MaterialInstanceDynamic))))))

(event Custom|SetSpeedColor
  (Rendering|Material|SetVectorParameterValue (stale EventBeginPlay _output_get_3) "EmissionColor" "(R=0.969378,G=1.000000,B=0.037684,A=1.000000)" :!class /Script/Engine.MaterialInstanceDynamic))

(event EventBeginPlay
  (Utilities|FlowControl|Sequence
    (:then_0
      (bind _returnvalue (Rendering|Material|CreateDynamicMaterialInstance (Variables|Default|GetTorus_001) 0 "/Game/Materials/dissolve_Inst.dissolve_Inst" "None" :!class /Script/Engine.PrimitiveComponent))
      (bind _output_get (Variables|Default|SetDM_torus_1 _returnvalue)))
    (:then_1
      (bind _returnvalue_2 (Rendering|Material|CreateDynamicMaterialInstance (Variables|Default|GetTorus) 0 "/Game/Materials/dissolve_Inst.dissolve_Inst" "None" :!class /Script/Engine.PrimitiveComponent))
      (bind _output_get_2 (Variables|Default|SetDM_Torus_2 _returnvalue_2)))
    (:then_2
      (bind _returnvalue_3 (Rendering|Material|CreateDynamicMaterialInstance (Variables|Default|GetSphere) 0 "/Game/Materials/dissolve_Inst.dissolve_Inst" "None" :!class /Script/Engine.PrimitiveComponent))
      (bind _output_get_3 (Variables|Default|SetDM_Sphere _returnvalue_3)))))

(fn ConstructionScript)