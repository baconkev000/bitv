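; Base projectile actor that flies at a configurable speed and destroys itself on impact.
; The construction script copies Speed into the projectile movement's initial and maximum speed, and also assigns a Gravity value.
; At BeginPlay its box collision ignores the owner during movement.
; A box hit broadcasts the OnProjectileImpact dispatcher with the other actor and hit result before the projectile is destroyed.
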(event OnComponentHit(Box)
  (params (HitComponent :type Primitive%20Component%20Object%20Reference) (OtherActor :type Actor%20Object%20Reference) (OtherComp :type Primitive%20Component%20Object%20Reference) (NormalImpulse :type Vector :default "0, 0, 0") (Hit :type Hit%20Result%20Structure%20%28by%20ref%29))
  (Default|CallOnProjectileImpact OtherActor Hit)
  (Actor|DestroyActor))

(event EventBeginPlay
  (Collision|IgnoreActorwhenMoving (Variables|Default|GetBox) (Components|GetOwner) true))

(fn ConstructionScript
  (bind _projectilemovement (Variables|Default|GetProjectileMovement))
  (bind _speed (Variables|ProjectileSettings|GetSpeed))
  (Variables|/Script/Engine.ProjectileMovementComponent|SetInitialSpeed _projectilemovement _speed)
  (Variables|/Script/Engine.ProjectileMovementComponent|SetMaxSpeed _projectilemovement _speed)
  (Variables|ProjectileSettings|SetGravity (Variables|ProjectileSettings|GetGravity)))