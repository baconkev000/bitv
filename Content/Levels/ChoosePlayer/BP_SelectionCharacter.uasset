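; BP_SelectionCharacter is the preview actor for choosing a player character in the ChoosePlayer level.
; Its ChangeCharacter event steps through the Characters array, wrapping back to the first entry, and applies that mesh to its SkeletalMesh component.
; It then stores the chosen mesh in the GI_Selection game instance as SkeletalMeshSelected.
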(event Custom|ChangeCharacter
  (if (< (Variables|Default|GetCurrentCharacterIndex) (- (Utilities|Array|Length (Variables|Default|GetCharacters)) 1))
    (Math|Integer|IncrementInt (Variables|Default|GetCurrentCharacterIndex)
      (:%20%20
        _))
    (else
      (Variables|Default|SetCurrentCharacterIndex 0)))
  (Components|SkeletalMesh|SetSkeletalMeshAsset (Variables|Default|GetSkeletalMesh) (Utilities|Array|Get(acopy) (Variables|Default|GetCharacters) (Variables|Default|GetCurrentCharacterIndex)))
  (bind _asgi_selection (Utilities|Casting|CastToGI_Selection (Game|GetGameInstance)))
  (Variables|/Game/Levels/GI_Selection.GI_Selection_C|SetSkeletalMeshSelected _asgi_selection (Utilities|Array|Get(acopy) (Variables|Default|GetCharacters) (Variables|Default|GetCurrentCharacterIndex))))

(event EventBeginPlay)

(event Collision|EventActorBeginOverlap
  (params (OtherActor :type Actor%20Object%20Reference)))

(event EventTick
  (params (DeltaSeconds :type Float%20%28single-precision%29)))

(fn ConstructionScript)