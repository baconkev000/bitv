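; Enemy alien character Blueprint that handles taking damage and dying.
; Any damage reduces Health, and reaching zero or below sets a one-time IsDying guard and halts character movement.
; Death plays a random section of the dying-alien montage from DeathAnims, with a montage notify triggering a sound at the actor's location.
; The actor is destroyed when the montage blends out.
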(event Game|Damage|EventAnyDamage
  (params (Damage :type Float%20%28single-precision%29) (DamageType :type Damage%20Type%20Object%20Reference) (InstigatedBy :type Controller%20Object%20Reference) (DamageCauser :type Actor%20Object%20Reference))
  (bind _deathanims (Variables|Default|GetDeathAnims))
  (if (> (- (Variables|Default|GetHealth) Damage) 0.0)
    (Variables|Default|SetHealth (- (Variables|Default|GetHealth) Damage))
    (else
      (Variables|Default|SetHealth (- (Variables|Default|GetHealth) Damage))
      (if (not (Variables|Default|GetIsDying))
        (Variables|Default|SetIsDying true)
        (Components|Movement|StopMovementImmediately (Variables|Character|GetCharacterMovement))
        (Animation|Montage|PlayMontage (Variables|Character|GetMesh) "/Game/Characters/Alien/AnimMontages/AM_DyingAlien.AM_DyingAlien" 1.0 0.0 (Utilities|String|StringToName (Utilities|Array|Get(acopy) _deathanims (Math|Random|RandomIntegerinRange 0 (- (Utilities|Array|Length _deathanims) 1))))
          (:OnBlendOut
            (Actor|DestroyActor))
          (:OnNotifyBegin
            (Audio|PlaySoundatLocation "/Game/Music/AlienProwls.AlienProwls" (Transformation|GetActorLocation) "0, 0, 0" 1.0 1.0 0.0 0 0 0 0)))))))

(fn ConstructionScript)