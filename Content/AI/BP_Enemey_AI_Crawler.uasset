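; Alien crawler enemy AI that roams random reachable points, chases players it sees and plays periodic prowl sounds.
; PawnSensing switches it to a faster AIMoveTo chase, and a retriggerable delay returns it to roaming after sightings stop.
; Reaching the target triggers an RPC-named punch montage unless crawling, a state also passed to the AnimBP.
; Lethal damage stops movement, plays a random death montage section, then destroys the actor.
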(event OnSeePawn(PawnSensing)
  (params (Pawn :type Pawn%20Object%20Reference))
  (Utilities|Casting|CastToBP_ThirdPersonCharacter Pawn)
  (if (not (Variables|Default|GetIsDying))
    (Variables|/Script/Engine.CharacterMovementComponent|SetMaxWalkSpeed (Variables|Character|GetCharacterMovement) (Variables|Default|GetHoldMaxSpeed))
    (Variables|Default|SetIsRoaming false)
    (Utilities|FlowControl|Sequence
      (:then_0
        (Variables|Default|SetisSeeingPlayer true)
        (CallFunction|FollowPlayer))
      (:then_1
        (Utilities|FlowControl|RetriggerableDelay 3.0)
        (Variables|Default|SetIsRoaming true)
        (CallFunction|RandomRoam)))))

(event Custom|FollowPlayer
  (if (not (Variables|Default|GetIsDying))
    (Variables|Default|SetcanAttack true)
    (if (Variables|Default|GetisSeeingPlayer)
      (AI|AIMoveTo self "0, 0, 0" (stale OnSeePawn(PawnSensing) Pawn) 7e+01 false
        (:OnSuccess
          (if (Variables|Default|GetcanAttack)
            (Variables|Default|SetcanAttack false)
            (if (not (Variables|Default|GetIsCrawling))
              (CallFunction|RPCServerAttackAnim)))))
      (else
        (Variables|Default|SetisSeeingPlayer false)))))

(event Custom|RPC_AttackAnim
  (bind _returnvalue (Animation|PlayAnimMontage "/Game/Characters/Alien/AnimMontages/AM_AI_punch.AM_AI_punch" 1.0 "None"))
  (Audio|PlaySoundatLocation "/Game/Music/AlienStrikes.AlienStrikes" (Transformation|GetActorLocation) "0, 0, 0" 1.0 1.0 0.0 0 0 0 0)
  (Utilities|FlowControl|Delay _returnvalue)
  (Variables|Default|SetcanAttack true))

(event Custom|PlayAlienSound
  (Utilities|Time|SetTimerbyEvent (delegate Custom|PlayAlienSound) (Math|Random|RandomFloatinRange 5.0 15.0) true false 5.0)
  (Audio|PlaySoundatLocation "/Game/Music/AlienProwls.AlienProwls" (Transformation|GetActorLocation) "0, 0, 0" 1.0 1.0 0.0 0 0 0 0))

(event Custom|Random%20Roam
  (if (not (Variables|Default|GetIsDying))
    (Variables|/Script/Engine.CharacterMovementComponent|SetMaxWalkSpeed (Variables|Character|GetCharacterMovement) (Variables|Default|GetRoamSpeed))
    (AI|AIMoveTo self (.RandomLocation (AI|Navigation|GetRandomReachablePointinRadius (Transformation|GetActorLocation) 1e+03 0 0)) 0 5.0 false
      (:OnSuccess
        (Utilities|FlowControl|Delay 0.2)
        (CallFunction|RandomRoam)))))

(event Custom|RPC_Server_Attack_Anim
  (CallFunction|RPCAttackAnim))

(event Game|Damage|EventAnyDamage
  (params (Damage :type Float%20%28single-precision%29) (DamageType :type Damage%20Type%20Object%20Reference) (InstigatedBy :type Controller%20Object%20Reference) (DamageCauser :type Actor%20Object%20Reference))
  (bind _deathanims (Variables|Default|GetDeathAnims))
  (if (> (- (Variables|Default|GetHealth) Damage) 0.0)
    (Variables|Default|SetHealth (- (Variables|Default|GetHealth) Damage))
    (else
      (Variables|Default|SetHealth (- (Variables|Default|GetHealth) Damage))
      (if (not (Variables|Default|GetIsDying))
        (Variables|Default|SetIsDying true)
        (Components|Movement|StopMovementImmediately (Variables|Character|GetCharacterMovement))
        (Animation|Montage|PlayMontage (Variables|Character|GetMesh) "/Game/Characters/Alien/AnimMontages/AM_DyingAlien.AM_DyingAlien" 1.0 0.0 (Utilities|String|StringToName (Utilities|Array|Get(acopy) _deathanims (Math|Random|RandomIntegerinRange 0 (- (Utilities|Array|Length _deathanims) 1))))
          (:OnBlendOut
            (Actor|DestroyActor))
          (:OnNotifyBegin
            (Audio|PlaySoundatLocation "/Game/Music/AlienProwls.AlienProwls" (Transformation|GetActorLocation) "0, 0, 0" 1.0 1.0 0.0 0 0 0 0)))))))

(event EventBeginPlay
  (if (Variables|Default|GetIsCrawling)
    (bind _asabp_alien (Utilities|Casting|CastToABP_alien (Components|SkeletalMesh|GetAnimInstance (Variables|Character|GetMesh))))
    (Variables|/Game/Characters/Alien/ABP_alien.ABP_alien_C|SetIsCrawling _asabp_alien (Variables|Default|GetIsCrawling)))
  (CallFunction|PlayAlienSound)
  (if (not (Variables|Default|GetisSeeingPlayer))
    (Variables|Default|SetIsRoaming true)
    (CallFunction|RandomRoam)))

(fn ConstructionScript)